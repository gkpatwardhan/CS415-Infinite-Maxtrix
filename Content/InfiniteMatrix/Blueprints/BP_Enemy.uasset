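; BP_Enemy is an enemy actor that damages the player on contact and awards score when shot.
; All logic runs in the Enemy component's hit event, branching on what it struck.
; Hitting BP_Player lowers clamped Health, triggers the restart display and death flag at zero, then destroys the enemy.
; Hitting BP_Player_Projectile increases the score through the projectile's Player reference, then destroys both enemy and projectile.
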(event `self.Enemy.OnComponentHit`
  (params (HitComponent :type "PrimitiveComponent Object Reference") (OtherActor :type "Actor Object Reference") (OtherComp :type "PrimitiveComponent Object Reference") (NormalImpulse :type "Vector Structure") (Hit :type "HitResult Structure (by ref)"))
  ;[1 1 1] Enemy 1 Collision Detection
  (`|ExecutionSequence`
    (:`then_0`
      (bind _asbp_player (cast `/Game/InfiniteMatrix/Blueprints/BP_Player` OtherActor))
      (bind _output_get (set `/Game/InfiniteMatrix/Blueprints/BP_Player.Health` (`KismetMathLibrary.FClamp` (- (`/Game/InfiniteMatrix/Blueprints/BP_Player.Health` _asbp_player) 10.0) 0.0 100.0) _asbp_player))
      (if (<= _output_get 0.0)
        (`/Game/InfiniteMatrix/Blueprints/BP_Player.DisplayRestart` _asbp_player)
        (set `/Game/InfiniteMatrix/Blueprints/BP_Player.IsDead` true _asbp_player))
      (`self.K2_DestroyActor`))
    (:`then_1`
      (bind _asbp_player_projectile (cast `/Game/InfiniteMatrix/Blueprints/BP_Player_Projectile` OtherActor))
      (`/Game/InfiniteMatrix/Blueprints/BP_Player.Increase Score` (`/Game/InfiniteMatrix/Blueprints/BP_Player_Projectile.Player` _asbp_player_projectile) 10.0)
      (`self.K2_DestroyActor`)
      (`self.K2_DestroyActor` _asbp_player_projectile))))

(fn `UserConstructionScript`)