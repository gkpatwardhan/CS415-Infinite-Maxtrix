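; BP_Tunnel is an endless-runner tunnel segment with a rotating holed wall that the player passes through.
; Clearing the trigger awards score, has TunnelSpawner spawn another segment and destroys this one.
; Wall hits cost health and shake the camera, replacing the segment or showing restart on death; gift packs heal, and both absorb projectiles.
; Randomize functions, not called here, vary wall mesh and angle, gift placement and enemy spawns.
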(event `self.ReceiveTick`
  (params (DeltaSeconds :type "Float (single-precision)"))
  ;[1 1 1] Tunnnel rotation
  (`SceneComponent.K2_AddLocalRotation` (`self.WallMesh`) (`KismetMathLibrary.MakeRotator` (* DeltaSeconds (`self.RotateSpeed`))) false false))

(event `self.TriggerZone.OnComponentBeginOverlap`
  (params (OverlappedComponent :type "PrimitiveComponent Object Reference") (OtherActor :type "Actor Object Reference") (OtherComp :type "PrimitiveComponent Object Reference") (OtherBodyIndex :type Integer) (bFromSweep :type Boolean) (SweepResult :type "HitResult Structure (by ref)"))
  (bind _gift_packs (`self.Gift packs`))
  ;[1 1 1] Trigger Zone
  (bind _asbp_player (cast `/Game/InfiniteMatrix/Blueprints/BP_Player` OtherActor))
  (`|ExecutionSequence`
    (:`then_0`
      (`/Game/InfiniteMatrix/Blueprints/BP_Player.Increase Score` _asbp_player 10.0))
    (:`then_1`
      (`/Game/InfiniteMatrix/Blueprints/BP_TunnelSpawner.SpawnTunnelAtSpawnPoint` (`self.TunnelSpawner`)))
    (:`then_2`
      (`/Engine/EditorBlueprintResources/StandardMacros.IsValid` _gift_packs
        (:`Is Valid`
          (`ActorComponent.K2_DestroyComponent` _gift_packs))))
    (:`then_3`
      (for _array_element (`|MakeArray` null :!type "Object Object Reference")
        (`/Engine/EditorBlueprintResources/StandardMacros.IsValid` _array_element
          (:`Is Valid`
            (bind _asactor_component (cast `ActorComponent` _array_element))
            (`ActorComponent.K2_DestroyComponent` _asactor_component)))))
    (:`then_4`
      (`self.K2_DestroyActor`))))

(event `self.WallMesh.OnComponentHit`
  (params (HitComponent :type "PrimitiveComponent Object Reference") (OtherActor :type "Actor Object Reference") (OtherComp :type "PrimitiveComponent Object Reference") (NormalImpulse :type "Vector Structure") (Hit :type "HitResult Structure (by ref)"))
  ;[1 1 1] Wall Collision
  (`|ExecutionSequence`
    (:`then_0`
      (bind _asbp_player (cast `/Game/InfiniteMatrix/Blueprints/BP_Player` OtherActor))
      (`|ExecutionSequence`
        (:`then_0`
          (bind _output_get (set `/Game/InfiniteMatrix/Blueprints/BP_Player.Health` (`KismetMathLibrary.FClamp` (- (`/Game/InfiniteMatrix/Blueprints/BP_Player.Health` _asbp_player) 20.0) 0.0 100.0) _asbp_player))
          (if (<= _output_get 0.0)
            (set `/Game/InfiniteMatrix/Blueprints/BP_Player.IsDead` true _asbp_player)
            (`/Game/InfiniteMatrix/Blueprints/BP_Player.DisplayRestart` _asbp_player)
            (else
              (`/Game/InfiniteMatrix/Blueprints/BP_TunnelSpawner.SpawnTunnelAtSpawnPoint` (`self.TunnelSpawner`))
              (`self.K2_DestroyActor`))))
        (:`then_1`
          (`GameplayStatics.PlayWorldCameraShake` "/Game/InfiniteMatrix/Blueprints/BP_Camera_Shake.BP_Camera_Shake_C" (`self.K2_GetActorLocation` _asbp_player) 0.0 500.0))))
    (:`then_1`
      (bind _asbp_player_projectile (cast `/Game/InfiniteMatrix/Blueprints/BP_Player_Projectile` OtherActor))
      (`self.K2_DestroyActor` _asbp_player_projectile))))

(event `self.Gift packs.OnComponentHit`
  (params (HitComponent :type "PrimitiveComponent Object Reference") (OtherActor :type "Actor Object Reference") (OtherComp :type "PrimitiveComponent Object Reference") (NormalImpulse :type "Vector Structure") (Hit :type "HitResult Structure (by ref)"))
  ;[1 1 1] Gift pack collision
  (bind _asbp_player (cast `/Game/InfiniteMatrix/Blueprints/BP_Player` OtherActor)
    (:`then`
      (set `/Game/InfiniteMatrix/Blueprints/BP_Player.Health` (`KismetMathLibrary.FClamp` (+ (`/Game/InfiniteMatrix/Blueprints/BP_Player.Health` _asbp_player) 40.0) 0.0 100.0) _asbp_player)
      (`ActorComponent.K2_DestroyComponent` (`self.Gift packs`)))
    (:`CastFailed`
      (bind _asbp_player_projectile (cast `/Game/InfiniteMatrix/Blueprints/BP_Player_Projectile` OtherActor))
      (`self.K2_DestroyActor` _asbp_player_projectile))))

(fn `Get Random Position In Tunnel`
  (returns (Location :type "Vector Structure"))
  (bind _returnvalue (`KismetMathLibrary.RandomFloatInRange` 0.0 170.0))
  (bind _returnvalue_2 (`KismetMathLibrary.RandomFloatInRange` (* _returnvalue -1.0) _returnvalue))
  (return (`KismetMathLibrary.MakeVector` (`KismetMathLibrary.RandomFloatInRange` 0.0 2000.0) _returnvalue_2 (* (- _returnvalue (`KismetMathLibrary.Abs` _returnvalue_2)) (- (`KismetMathLibrary.RandomIntegerInRange` 0 2) 1)))))

(fn `Randomize Enemy`
  (for _ (range (+ (`KismetMathLibrary.RandomIntegerInRange` 0 3) 1))
    (bind _location (`self.Get Random Position In Tunnel`))
    (`|SpawnActorFromClass` "/Game/InfiniteMatrix/Blueprints/BP_Enemy.BP_Enemy_C" (`KismetMathLibrary.MakeTransform` (+ _location (`self.K2_GetActorLocation`)) (struct :`Yaw` 90.0) (5.0 5.0 5.0)) "Undefined" "OverrideRootScale" null null)))

(fn `Randomize Gift`
  (if (`KismetMathLibrary.RandomBool`)
    (`StaticMeshComponent.SetStaticMesh` (`self.Gift packs`) "/Game/InfiniteMatrix/Meshes/SM_Energy_1.SM_Energy_1")
    (bind _location (`self.Get Random Position In Tunnel`))
    (`SceneComponent.K2_SetRelativeLocation` (`self.Gift packs`) _location false false)))

(fn `RandomizeWall`
  (`StaticMeshComponent.SetStaticMesh` (`self.WallMesh`) (select `int` (`KismetMathLibrary.RandomIntegerInRange` 0 3) :`0` "/Game/InfiniteMatrix/Meshes/SM_Hole_01.SM_Hole_01" :`1` "/Game/InfiniteMatrix/Meshes/SM_Hole_02.SM_Hole_02" :`2` "/Game/InfiniteMatrix/Meshes/SM_Hole_03.SM_Hole_03" :`3` "/Game/InfiniteMatrix/Meshes/SM_Hole_04.SM_Hole_04" :!type "StaticMesh Object Reference"))
  (`SceneComponent.K2_AddLocalRotation` (`self.WallMesh`) (`KismetMathLibrary.MakeRotator` (`KismetMathLibrary.RandomFloatInRange` 0.0 360.0)) false false))

(fn `UserConstructionScript`)